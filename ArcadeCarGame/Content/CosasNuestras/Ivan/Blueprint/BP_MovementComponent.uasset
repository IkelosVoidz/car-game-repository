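; BP_MovementComponent is an actor component that drives its owner's physics body toward a target forward speed and yaw rate.
; On BeginPlay it caches the owner's root as a primitive component.
; Each tick it projects linear velocity on the forward vector and angular velocity on the up vector.
; It then applies force and torque proportional to the error from each target, acting as a simple proportional controller.
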(event EventBeginPlay
  (bind _asprimitive_component (Utilities|Casting|CastToPrimitiveComponent (Variables|/Script/Engine.Actor|GetRootComponent (Components|GetOwner))))
  (Variables|Default|SetRefToBody _asprimitive_component))

(event EventTick
  (params (DeltaSeconds :type Float%20%28single-precision%29))
  (bind _reftobody (Variables|Default|GetRefToBody))
  (bind _reftobody_2 (Variables|Default|GetRefToBody))
  (bind _reftobody_3 (Variables|Default|GetRefToBody))
  (bind _reftobody_4 (Variables|Default|GetRefToBody)
    (:then
      (bind _returnvalue (Physics|GetPhysicsLinearVelocity _reftobody_4 "None"))
      (Variables|Default|SetCurrentSpeed (Math|Vector|DotProduct _returnvalue (Math|Vector|GetForwardVector _reftobody_4)))
      (Variables|Default|SetCurrentAngularSpeed (Math|Vector|DotProduct (Physics|GetPhysicsAngularVelocityinDegrees _reftobody "None") (Math|Vector|GetUpVector _reftobody)))
      (Physics|AddForce _reftobody_2 (* (Math|Vector|GetForwardVector _reftobody_2) (* (- (Variables|Default|GetTargetSpeed) (Variables|Default|GetCurrentSpeed)) (Variables|Default|GetSpeed%20to%20Force%20Factor))) "None" false)
      (Class|PrimitiveComponent|AddTorqueinDegrees _reftobody_3 (* (Math|Vector|GetUpVector _reftobody_3) (* (- (Variables|Default|GetTargetAngularSpeed) (Variables|Default|GetCurrentAngularSpeed)) (Variables|Default|GetAngularSpeedToTorqueFactor))) "None" false))
    (:else)))