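; Nitro boost component that pushes a target along its forward vector while managing a limited nitro gauge.
; The Nitro event applies force when input and charge allow or Infinite is set, and starts a cooldown once the gauge is empty.
; Tick drains or refills the gauge per frame without delta-time scaling, prints it, and ends cooldown once it exceeds half capacity.
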(event Custom|Nitro
  (params (ActorToAffect :type Primitive%20Component%20Object%20Reference) (Input :type Boolean))
  (bind _infinite (Variables|Checks|GetInfinite))
  (bind _nitrocurrentamount (Variables|NitroParams|GetNitroCurrentAmount))
  (bind _returnvalue (> _nitrocurrentamount 0.0))
  (bind _returnvalue_2 (and Input _returnvalue))
  (bind _returnvalue_3 (or _infinite _returnvalue_2))
  (if (not (Variables|Checks|GetCooldownActive))
    (Variables|Checks|SetNitroActive _returnvalue_3)
    (if _returnvalue_3
      (CallFunction|AddBoost ActorToAffect (Variables|NitroParams|GetNitroForce))
      (Development|PrintString "Nitro!")
      (elif (not _returnvalue)
        (Variables|Checks|SetCooldownActive true)))))

(event EventBeginPlay
  (Variables|NitroParams|SetNitroCurrentAmount (Variables|NitroParams|GetNitroMaxAmount)))

(event EventTick
  (params (DeltaSeconds :type Float%20%28single-precision%29))
  (Utilities|FlowControl|Sequence
    (:then_0
      (if (Variables|Checks|GetCooldownActive)
        (if (> (Variables|NitroParams|GetNitroCurrentAmount) (/ (Variables|NitroParams|GetNitroMaxAmount) 2.0))
          (Variables|Checks|SetCooldownActive false))))
    (:then_1
      (if (Variables|Checks|GetNitroActive)
        (CallFunction|NitroStep (* (Variables|NitroParams|GetNitroDecreaseAmount) -1.0) DeltaSeconds)
        (else
          (CallFunction|NitroStep (Variables|NitroParams|GetNitroIncreaseAmount) DeltaSeconds)))
      (Development|PrintString (Utilities|String|ToString(Float) (Variables|NitroParams|GetNitroCurrentAmount))))))

(fn AddBoost
  (params (Target :type Primitive%20Component%20Object%20Reference) (BoostForce :type Float%20%28double-precision%29))
  (Physics|AddForce Target (* (Math|Vector|GetForwardVector Target) BoostForce 1e+03) "None" false))

(fn NitroStep
  (params (Step :type Float%20%28double-precision%29) (Delta :type Float%20%28double-precision%29))
  (Variables|NitroParams|SetNitroCurrentAmount (Math|Float|Clamp(Float) (+ (Variables|NitroParams|GetNitroCurrentAmount) Step) 0.0 (Variables|NitroParams|GetNitroMaxAmount))))