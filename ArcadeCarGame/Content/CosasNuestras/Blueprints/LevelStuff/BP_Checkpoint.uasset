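; Level checkpoint actor that signals it has been cleared when an actor exits its Trigger volume moving along the checkpoint's Direction.
; On end overlap it hides the trigger and disables its overlaps, even if the direction check then fails.
; A positive dot product of velocity and Direction's forward vector calls CheckpointCleared, passing the checkpoint number and the actor's transform raised slightly in Z.
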(event OnComponentEndOverlap(Trigger)
  (params (OverlappedComponent :type Primitive%20Component%20Object%20Reference) (OtherActor :type Actor%20Object%20Reference) (OtherComp :type Primitive%20Component%20Object%20Reference) (OtherBodyIndex :type Integer))
  (bind _returnvalue (Transformation|GetActorLocation))
  (bind _trigger (Variables|Default|GetTrigger))
  (Development|SetHiddeninGame _trigger true false)
  (Variables|/Script/Engine.PrimitiveComponent|SetbGenerateOverlapEvents _trigger false)
  (if (> (Math|Vector|DotProduct (Transformation|GetVelocity OtherActor) (Math|Rotator|GetRotationXVector (Transformation|GetWorldRotation (Variables|Default|GetDirection)))) 0.0)
    (Default|CallCheckpointCleared (Variables|Default|GetCheckpointNumber) (Math|Transform|MakeTransform (Math|Vector|MakeVector (.x _returnvalue) (.y _returnvalue) (+ (.z _returnvalue) 1e+02)) (Transformation|GetActorRotation)))))

(fn ConstructionScript)