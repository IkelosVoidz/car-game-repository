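; Race game instance that owns the save data, keeping best race and lap times keyed by race name.
; On init it synchronously loads the BP_MySaveGame slot, or creates a new save object if none exists.
; SaveRace writes a race entry and saves the slot, while getters return the whole save or one race's record.
; Saving and loading support sync or async, but only a completed async load calls OnGameLoaded.
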(event EventInit
  (CallFunction|LoadGameData false))

(event EventSaveGameData
  (params (isAsync :type Boolean))
  (bind _slotname (Variables|Default|GetSlotName))
  (bind _savedgamedata (Variables|Default|GetSavedGameData))
  ;[0.224 0.224 0.224] Save Game
  (if isAsync
    (|AsyncSaveGametoSlot _savedgamedata _slotname)
    (else
      (SaveGame|SaveGametoSlot _savedgamedata _slotname))))

(event EventLoadGameData
  (params (isAsync :type Boolean))
  (bind _slotname (Variables|Default|GetSlotName))
  ;[0.1198 0.1198 0.1198] Load Game
  (bind _returnvalue (SaveGame|DoesSaveGameExist (Variables|Default|GetSlotName)))
  (if _returnvalue
    (if isAsync
      (bind _savegame (|AsyncLoadGamefromSlot _slotname)
        (:Completed
          (bind _asbp_my_save_game (Utilities|Casting|CastToBP_MySaveGame _savegame))
          (Variables|Default|SetSavedGameData _asbp_my_save_game)
          (Default|CallOnGameLoaded)))
      (else
        (bind _returnvalue_2 (SaveGame|LoadGamefromSlot _slotname))
        (bind _asbp_my_save_game_2 (Utilities|Casting|CastToBP_MySaveGame _returnvalue_2))
        (Variables|Default|SetSavedGameData _asbp_my_save_game_2)))
    (else
      (bind _returnvalue_3 (SaveGame|CreateSaveGameObject "/Game/CosasNuestras/Blueprints/SaveGame/BP_MySaveGame.BP_MySaveGame_C"))
      (Variables|Default|SetSavedGameData _returnvalue_3))))

(event EventSaveRace
  (params (RaceSave :type S%20Race%20Save%20Structure) (RaceName :type String) (isAsync :type Boolean))
  (bind _savedgamedata (Variables|Default|GetSavedGameData))
  (Utilities|Map|Add (.racesaves (Variables|/Game/CosasNuestras/Blueprints/SaveGame/BP_MySaveGame.BP_MySaveGame_C|GetSaveGame _savedgamedata)) RaceName (Utilities|Struct|MakeS_RaceSave (.bestracetime RaceSave) (.bestlaptime RaceSave)))
  (Variables|/Game/CosasNuestras/Blueprints/SaveGame/BP_MySaveGame.BP_MySaveGame_C|SetSaveGame _savedgamedata (Utilities|Struct|MakeS_SaveStructure (.racesaves (Variables|/Game/CosasNuestras/Blueprints/SaveGame/BP_MySaveGame.BP_MySaveGame_C|GetSaveGame _savedgamedata))))
  (CallFunction|SaveGameData isAsync))

(fn GetGameData
  (return (Variables|Default|GetSavedGameData)))

(fn GetRaceData
  (params (RaceName :type String))
  (bind _savedgamedata (Variables|Default|GetSavedGameData))
  (bind _savegame (Variables|/Game/CosasNuestras/Blueprints/SaveGame/BP_MySaveGame.BP_MySaveGame_C|GetSaveGame _savedgamedata))
  (bind (_value _returnvalue) (Utilities|Map|Find (.racesaves _savegame) RaceName))
  (if _returnvalue
    _
    (else
      (Development|PrintString (Utilities|String|ToString(Text) (Utilities|Text|FormatText "Couldnt find save with map name = {mapname}" RaceName)))))
  (return _value))