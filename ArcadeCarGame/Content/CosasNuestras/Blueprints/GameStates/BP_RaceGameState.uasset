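; Race game state that tracks lap count, lap and race times, loading the best times from the game instance on BeginPlay.
; Two timelines serve as clocks, and UpdateLap increments the lap and checks its time against the best before restarting the lap timer.
; Once RaceComplete is set, only a matching or better race time saves both records, stops the race timer and triggers a provisional delayed level restart.
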(event Custom|StartRaceTime
  ;[0.1096 0.9103 1] Race Timers
  (bind _time (Timeline|RaceTime Play)
    (:Update
      (Variables|RaceStats|SetCurrentRaceTime _time))))

(event Custom|StopRaceTime
  ;[0.1096 0.9103 1] Race Timers
  (bind _time (Timeline|RaceTime Stop)
    (:Update
      (Variables|RaceStats|SetCurrentRaceTime _time))))

(event Custom|StartLapTime
  ;[0.1096 0.9103 1] Race Timers
  (bind _time (Timeline|LapTime Play)
    (:Update
      (Variables|RaceStats|SetCurrentLapTime _time))))

(event Custom|StopLapTime
  ;[0.1096 0.9103 1] Race Timers
  (bind _time (Timeline|LapTime Stop)
    (:Update
      (Variables|RaceStats|SetCurrentLapTime _time))))

(event Custom|RestartLevel
  ;[1 1 1] Provisional
  (Utilities|FlowControl|Delay 1.0)
  (Development|ExecuteConsoleCommand "RestartLevel" 0))

(event Custom|Update%20Lap
  ;[1 1 1] Sequence of update lap (ends with restart if race complete is true)
  (if (Variables|RaceChecks|GetRaceComplete)
    _
    (else
      (bind _result (Math|Integer|IncrementInt (Variables|RaceStats|GetCurrentLap))
        (:%20%20
          _))))
  (CallFunction|LapTimeCheck)
  (Development|PrintString (Utilities|String|ToString(Integer) _result)))

(event EventBeginPlay
  (bind _racedata (Class|BPISaveGame|GetRaceData(Message) (Game|GetGameInstance)))
  (Variables|RaceStats|SetBestRaceTime (.bestracetime _racedata))
  (Variables|RaceStats|SetBestLapTime (.bestlaptime _racedata))
  (CallFunction|StartRaceTime)
  (CallFunction|StartLapTime))

(fn ConstructionScript)

(fn UpdateLap)

(fn LapTimeCheck
  (CallFunction|StopLapTime)
  (if (<= (Variables|RaceStats|GetCurrentLapTime) (Variables|RaceStats|GetBestLapTime))
    (bind _output_get (Variables|RaceStats|SetBestLapTime (Variables|RaceStats|GetCurrentLapTime)))
    (Development|PrintString (Class|KismetStringLibrary|TimeSecondstoString _output_get))
    (Variables|RaceStats|SetCurrentLapTime 0.0)
    (else
      (Variables|RaceStats|SetCurrentLapTime 0.0)))
  (if (Variables|RaceChecks|GetRaceComplete)
    (CallFunction|RaceTimeCheck)
    (else
      (CallFunction|StartLapTime))))

(fn RaceTimeCheck
  (if (<= (Variables|RaceStats|GetCurrentRaceTime) (Variables|RaceStats|GetBestRaceTime))
    (bind _output_get (Variables|RaceStats|SetBestRaceTime (Variables|RaceStats|GetCurrentRaceTime)))
    (Development|PrintString (Class|KismetStringLibrary|TimeSecondstoString _output_get))
    (Class|BPISaveGame|SaveRace(Message) (Game|GetGameInstance) (Utilities|Struct|MakeS_RaceSave (Variables|RaceStats|GetBestRaceTime) (Variables|RaceStats|GetBestLapTime)) false)
    (CallFunction|StopRaceTime)
    ;[1 1 1] Provisional
    (CallFunction|RestartLevel)))