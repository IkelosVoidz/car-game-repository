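; Player controller for a Chaos wheeled vehicle that feeds driving data to the vehicle HUD.
; On BeginPlay it casts the controlled pawn to WheeledVehiclePawn and caches its vehicle movement component.
; Every tick it passes that component's forward speed and current gear to the VehicleHud.
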(event EventBeginPlay
  ;[1 1 1] Setting Vehicle Movement Component from posessed pawn
  (|CallParentFunction)
  (bind _aswheeled_vehicle_pawn (Utilities|Casting|CastToWheeledVehiclePawn (Pawn|GetControlledPawn)))
  (Variables|Default|SetVehicle%20Movement%20Component (Variables|/Script/ChaosVehicles.WheeledVehiclePawn|GetVehicleMovementComponent _aswheeled_vehicle_pawn)))

(event EventTick
  (params (DeltaSeconds :type Float%20%28single-precision%29))
  ;[1 1 1] Update Vehicle UI
  (Default|UpdateSpeed (Variables|Default|GetVehicleHud) (Vehicle|GetForwardSpeed (Variables|Default|GetVehicle%20Movement%20Component)))
  (Default|UpdateGear (Variables|Default|GetVehicleHud) (Class|ChaosVehicleMovementComponent|GetCurrentGear (Variables|Default|GetVehicle%20Movement%20Component))))

(fn ConstructionScript
  (|CallParentFunction))