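; Hover suspension scene component that pushes its owner's physics-simulating root body up from the component's location, for use on BP_HoverVehicle.
; Each tick a downward trace measures compression over HoverDistance, and a spring-damper force (Stiffness, Damping from compression rate) is applied at that point.
; A second, longer trace sets the vehicle's IsInAir flag.
; One second after BeginPlay it attaches a test particle system to the body.
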(event Custom|doSomethingJEJE
  (Niagara|SpawnSystemAttached "/Game/CosasNuestras/Ivan/Blueprint/Test_Particles.Test_Particles" (Variables|Default|GetRefToBody) "None" "0, 0, 0" "0, 0, 0" "KeepRelativeOffset" false))

(event EventBeginPlay
  (Utilities|FlowControl|Sequence
    (:then_0
      (bind _asprimitive_component (Utilities|Casting|CastToPrimitiveComponent (Variables|/Script/Engine.Actor|GetRootComponent (Components|GetOwner))))
      (bind _output_get (Variables|Default|SetRefToBody _asprimitive_component))
      (if (not (Physics|IsSimulatingPhysics _output_get "None"))
        (Variables|Default|SetRefToBody 0)))
    (:then_1
      (Utilities|Time|SetTimerbyEvent (delegate Custom|doSomethingJEJE) 1.0))))

(event EventTick
  (params (DeltaSeconds :type Float%20%28single-precision%29))
  (bind _returnvalue (Components|GetOwner))
  (bind _returnvalue_2 (Transformation|GetWorldLocation))
  (bind _returnvalue_3 (Transformation|GetWorldLocation))
  (bind _hoverdistance (Variables|Default|GetHoverDistance))
  (Utilities|FlowControl|Sequence
    (:then_0
      (Variables|Default|GetRefToBody
        (:then
          (bind (_outhit _returnvalue_4) (Collision|LineTraceByChannel _returnvalue_2 (- _returnvalue_2 (* (Math|Vector|GetUpVector) (Variables|Default|GetHoverDistance))) "TraceTypeQuery1" false (Utilities|Array|MakeArray (Components|GetOwner)) "None"))
          (if _returnvalue_4
            (Variables|Default|SetHoverForce (+ (* (/ (- (/ (- _hoverdistance (.Distance (Collision|BreakHitResult _outhit))) _hoverdistance) (Variables|Default|GetPreviousCompression)) (Utilities|Time|GetWorldDeltaSeconds)) (Variables|Default|GetDamping)) (* (/ (- _hoverdistance (.Distance (Collision|BreakHitResult _outhit))) _hoverdistance) (Variables|Default|GetStiffness))))
            (Variables|Default|SetPreviousCompression (/ (- _hoverdistance (.Distance (Collision|BreakHitResult _outhit))) _hoverdistance))
            (Class|PrimitiveComponent|AddForceatLocation (Variables|Default|GetRefToBody) (* (Math|Vector|GetUpVector) (Variables|Default|GetHoverForce)) (Transformation|GetWorldLocation) "None")))
        (:else)))
    (:then_1
      (Variables|Default|GetRefToBody
        (:then
          (bind _returnvalue_5 (Collision|LineTraceByChannel _returnvalue_3 (- _returnvalue_3 (* (Math|Vector|GetUpVector) (+ (Variables|Default|GetHoverDistance) 3e+02))) "TraceTypeQuery1" false (Utilities|Array|MakeArray (Components|GetOwner)) "None"))
          (if _returnvalue_5
            (bind _asbp_hover_vehicle (Utilities|Casting|CastToBP_HoverVehicle _returnvalue))
            (Variables|/Game/CosasNuestras/Ivan/Blueprint/BP_HoverVehicle.BP_HoverVehicle_C|SetisInAir _asbp_hover_vehicle false)
            (else
              (bind _asbp_hover_vehicle_2 (Utilities|Casting|CastToBP_HoverVehicle _returnvalue))
              (Variables|/Game/CosasNuestras/Ivan/Blueprint/BP_HoverVehicle.BP_HoverVehicle_C|SetisInAir _asbp_hover_vehicle_2 true))))
        (:else)))))