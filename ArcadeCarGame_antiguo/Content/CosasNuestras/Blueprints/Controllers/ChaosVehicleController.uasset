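; Vehicle controller that feeds the possessed Chaos vehicle's speed and gear to its HUD.
; On BeginPlay it casts the controlled pawn to WheeledVehiclePawn and caches its VehicleMovementComponent.
; Each Tick, if the VehicleHud reference is valid, it passes the component's forward speed and current gear to the HUD.
; VehicleHud is not created or assigned in these graphs.
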(event EventBeginPlay
  ;[1 1 1] Setting Vehicle Movement Component from posessed pawn
  (|CallParentFunction)
  (bind _aswheeled_vehicle_pawn (Utilities|Casting|CastToWheeledVehiclePawn (Pawn|GetControlledPawn)))
  (Variables|Default|SetVehicle%20Movement%20Component (Variables|/Script/ChaosVehicles.WheeledVehiclePawn|GetVehicleMovementComponent _aswheeled_vehicle_pawn)))

(event EventTick
  (params (DeltaSeconds :type Float%20%28single-precision%29))
  (bind _vehiclehud (Variables|Default|GetVehicleHud))
  (bind _vehiclehud_2 (Variables|Default|GetVehicleHud))
  ;[1 1 1] Update Vehicle UI
  (Utilities|IsValid _vehiclehud_2
    (:Is%20Valid
      (Default|UpdateSpeed _vehiclehud_2 (Vehicle|GetForwardSpeed (Variables|Default|GetVehicle%20Movement%20Component)))
      (Utilities|IsValid _vehiclehud
        (:Is%20Valid
          (Default|UpdateGear _vehiclehud (Class|ChaosVehicleMovementComponent|GetCurrentGear (Variables|Default|GetVehicle%20Movement%20Component))))))))

(fn ConstructionScript
  (|CallParentFunction))