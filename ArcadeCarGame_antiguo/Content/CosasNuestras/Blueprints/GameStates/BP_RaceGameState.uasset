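; Race game state that tracks laps, current lap and race times, and per-level best times.
; On BeginPlay it loads bests from the GameInstance by level name and starts two Timelines used as stopwatches.
; UpdateLap advances the lap and records a faster lap; on race completion it checks the race best, saves both bests and stops the race timer.
; Provisional restart, save-reset and debug-print events are also included.
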(event Custom|Reset%20Saved%20Stats
  ;[1 1 1] Reset Saved Stats
  (Variables|RaceStats|SetBestRaceTime 0.0)
  (Variables|RaceStats|SetBestRaceTime 0.0)
  (bind _returnvalue (Game|GetCurrentLevelName true))
  (Class|BPISaveGame|SaveRace(Message) (Game|GetGameInstance) (Utilities|Struct|MakeS_RaceSave 0.0 0.0) _returnvalue false))

(event Custom|Show%20saved%20stats
  ;[1 1 1] Show all saved data
  (bind _save_game_data (Class|BPISaveGame|GetGameData(Message) (Game|GetGameInstance)))
  (bind _keys (Utilities|Map|Keys (.racesaves (Variables|/Game/CosasNuestras/Blueprints/SaveGame/BP_MySaveGame.BP_MySaveGame_C|GetSaveGame _save_game_data))))
  (for _array_element _keys
    (Development|PrintString (Utilities|String|Append _array_element "->" "    R:" (Class|KismetStringLibrary|TimeSecondstoString (.bestracetime (.Value (Utilities|Map|Find (.racesaves (Variables|/Game/CosasNuestras/Blueprints/SaveGame/BP_MySaveGame.BP_MySaveGame_C|GetSaveGame _save_game_data)) _array_element)))) "    L :" (Class|KismetStringLibrary|TimeSecondstoString (.bestlaptime (.Value (Utilities|Map|Find (.racesaves (Variables|/Game/CosasNuestras/Blueprints/SaveGame/BP_MySaveGame.BP_MySaveGame_C|GetSaveGame _save_game_data)) _array_element))))))))

(event Custom|StartRaceTime
  ;[0.1096 0.9103 1] Race Timers
  (bind _time (Timeline|RaceTime Play)
    (:Update
      (Variables|RaceStats|SetCurrentRaceTime _time))))

(event Custom|StopRaceTime
  ;[0.1096 0.9103 1] Race Timers
  (bind _time (Timeline|RaceTime Stop)
    (:Update
      (Variables|RaceStats|SetCurrentRaceTime _time))))

(event Custom|StartLapTime
  ;[0.1096 0.9103 1] Race Timers
  (bind _time (Timeline|LapTime Play)
    (:Update
      (Variables|RaceStats|SetCurrentLapTime _time))))

(event Custom|StopLapTime
  ;[0.1096 0.9103 1] Race Timers
  (bind _time (Timeline|LapTime Stop)
    (:Update
      (Variables|RaceStats|SetCurrentLapTime _time))))

(event Custom|RestartLevel
  ;[1 1 1] Provisional
  (Utilities|FlowControl|Delay 1.0)
  (Development|ExecuteConsoleCommand "RestartLevel" 0))

(event Custom|Update%20Lap
  ;[1 1 1] Sequence of update lap (ends with restart if race complete is true)
  (if (Variables|RaceChecks|GetRaceComplete)
    _
    (else
      (bind _result (Math|Integer|IncrementInt (Variables|RaceStats|GetCurrentLap))
        (:%20%20
          _))))
  (CallFunction|LapTimeCheck))

(event EventBeginPlay
  ;[1 1 1] Loading saved data of Current level
  (bind _returnvalue (Game|GetCurrentLevelName true))
  (bind _racedata (Class|BPISaveGame|GetRaceData(Message) (Game|GetGameInstance) _returnvalue))
  (bind _output_get (Variables|RaceStats|SetBestRaceTime (.bestracetime _racedata)))
  (bind _output_get_2 (Variables|RaceStats|SetBestLapTime (.bestlaptime _racedata)))
  (if (or (Math|Float|NearlyEqual(Float) _output_get_2 0.0 1e-06) (Math|Float|NearlyEqual(Float) _output_get 0.0 1e-06))
    (Variables|RaceChecks|SetFirstLapSave true)
    (Variables|RaceChecks|SetFirstRaceSave true))
  (Development|PrintString (Utilities|String|ToString(Boolean) (Variables|RaceChecks|GetFirstRaceSave)))
  (Development|PrintString (Utilities|String|ToString(Boolean) (Variables|RaceChecks|GetFirstLapSave)))
  (CallFunction|StartRaceTime)
  (CallFunction|StartLapTime))

(fn ConstructionScript)

(fn LapTimeCheck
  (CallFunction|StopLapTime)
  (if (Variables|RaceChecks|GetFirstLapSave)
    (Variables|RaceChecks|SetFirstLapSave false)
    (Variables|RaceStats|SetBestLapTime (Variables|RaceStats|GetCurrentLapTime) :!label _label)
    (elif (<= (Variables|RaceStats|GetCurrentLapTime) (Variables|RaceStats|GetBestLapTime))
      (goto _label)
      (else
        _)))
  (Variables|RaceStats|SetCurrentLapTime 0.0)
  (if (Variables|RaceChecks|GetRaceComplete)
    (CallFunction|RaceTimeCheck)
    (else
      (CallFunction|StartLapTime))))

(fn RaceTimeCheck
  (if (Variables|RaceChecks|GetFirstRaceSave)
    (Variables|RaceChecks|SetFirstRaceSave false)
    (Variables|RaceStats|SetBestRaceTime (Variables|RaceStats|GetCurrentRaceTime) :!label _label)
    (elif (<= (Variables|RaceStats|GetCurrentRaceTime) (Variables|RaceStats|GetBestRaceTime))
      (goto _label)
      (else
        _)))
  (bind _returnvalue (Game|GetCurrentLevelName true))
  (Development|PrintString "ESTTOY GUARDANDO AL ACABAR LA CARRERA")
  (Class|BPISaveGame|SaveRace(Message) (Game|GetGameInstance) (Utilities|Struct|MakeS_RaceSave (Variables|RaceStats|GetBestRaceTime) (Variables|RaceStats|GetBestLapTime)) _returnvalue false)
  ;[1 1 1] Provisional
  (CallFunction|StopRaceTime))

(fn RaceCompleteCheck
  (bind _output_get (Variables|RaceChecks|SetRaceComplete (>= (Variables|RaceStats|GetCurrentLap) (Variables|RaceStats|GetMaxLaps))))
  (return _output_get))