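; BP_VehicleState tracks the vehicle's respawn position based on checkpoint progress.
; On BeginPlay it sets RespawnPosition to the first player pawn's transform and binds to the cleared event of every BP_Checkpoint in the level.
; Each cleared checkpoint replaces RespawnPosition with the transform it reports.
; With no checkpoints it prints a warning and keeps the starting transform.
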(event Custom|Update%20Respawn%20Position
  (params (NextCheckpoint :type Integer) (Checkpoint%20Transform :type Transform))
  (Variables|Default|SetRespawn%20Position Checkpoint%20Transform))

(event EventBeginPlay
  (bind _outactors (Actor|GetAllActorsOfClass "/Game/CosasNuestras/Blueprints/LevelStuff/BP_Checkpoint.BP_Checkpoint_C"))
  (if (Utilities|Array|IsEmpty _outactors)
    (Development|PrintString "No checkpoints in level")
    (Variables|Default|SetRespawn%20Position (Transformation|GetActorTransform (Game|Player|GetPlayerPawn 0)) :!label _label)
    (else
      (for _array_element _outactors
        (EventDispatchers|BindEventtoCheckpointCleared _array_element (delegate Custom|Update%20Respawn%20Position))
        (goto _label)))))

(fn ConstructionScript)