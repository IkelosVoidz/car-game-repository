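; Vehicle component that provides a nitro boost backed by a limited, self-refilling charge.
; The Nitro event sets the active state from input and remaining charge, then AddBoost pushes the target along its forward vector with a scaled force.
; Tick drains or refills the clamped charge by a fixed amount per frame, ignoring delta time, and prints it for debugging.
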(event Custom|Nitro
  (params (ActorToAffect :type Primitive%20Component%20Object%20Reference) (Input :type Boolean))
  (Variables|Checks|SetNitroActive (and Input (> (Variables|NitroParams|GetNitroCurrentAmount) 0.0)))
  (if (Variables|Checks|GetOneTime)
    (Utilities|FlowControl|DoOnce false
      (:Completed
        _)))
  (CallFunction|AddBoost ActorToAffect (Variables|NitroParams|GetNitroForce))
  (Development|PrintString "Nitro!"))

(event EventBeginPlay
  (Variables|NitroParams|SetNitroCurrentAmount (Variables|NitroParams|GetNitroMaxAmount)))

(event EventTick
  (params (DeltaSeconds :type Float%20%28single-precision%29))
  (bind _nitroincreaseamount (Variables|NitroParams|GetNitroIncreaseAmount))
  (if (Variables|Checks|GetNitroActive)
    (CallFunction|NitroStep (* _nitroincreaseamount -1.0) DeltaSeconds)
    (else
      (CallFunction|NitroStep _nitroincreaseamount DeltaSeconds)))
  (Development|PrintString (Utilities|String|ToString(Float) (Variables|NitroParams|GetNitroCurrentAmount))))

(fn AddBoost
  (params (Target :type Primitive%20Component%20Object%20Reference) (BoostForce :type Float%20%28double-precision%29))
  (Physics|AddForce Target (* (Math|Vector|GetForwardVector Target) BoostForce 1e+03) "None" false))

(fn NitroStep
  (params (Step :type Float%20%28double-precision%29) (Delta :type Float%20%28double-precision%29))
  (Variables|NitroParams|SetNitroCurrentAmount (Math|Float|Clamp(Float) (+ (Variables|NitroParams|GetNitroCurrentAmount) Step) 0.0 (Variables|NitroParams|GetNitroMaxAmount))))